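; Orc1 is a flipbook-animated orc character that marches along its sprite's forward vector and attacks Walls it runs into.
; A capsule hit sets the attacking flag according to whether the other actor's class is exactly Wall.
; Tick prioritizes death, attack, idle and movement, stopping movement for the first three and clearing the attack flag after each use.
; Movement both adds input and directly forces velocity to max speed.
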(event OnComponentHit(CapsuleComponent)
  (params (HitComponent :type Primitive%20Component%20Object%20Reference) (OtherActor :type Actor%20Object%20Reference) (OtherComp :type Primitive%20Component%20Object%20Reference) (NormalImpulse :type Vector :default "0, 0, 0") (Hit :type Hit%20Result%20Structure%20%28by%20ref%29))
  (Variables|Default|SetIsAttacking (== (Utilities|GetClass OtherActor) "/Game/Blueprints/Wall/Wall.Wall_C")))

(event EventBeginPlay
  (|Animation))

(fn ConstructionScript)

(event EventTick
  (params (DeltaSeconds :type Float%20%28single-precision%29))
  (if (Variables|Default|GetDied)
    (Sprite|SetFlipbook (Variables|Default|GetSprite) (Variables|Animations|GetDiyng))
    (Components|Movement|StopMovementImmediately (Variables|Character|GetCharacterMovement))
    (elif (Variables|Default|GetIsAttacking)
      (Sprite|SetFlipbook (Variables|Default|GetSprite) (Variables|Animations|GetAttacking))
      (Variables|Default|SetIsAttacking false)
      (Variables|Default|SetIsIdle false)
      (Components|Movement|StopMovementImmediately (Variables|Character|GetCharacterMovement) :!label _label)
      (elif (Variables|Default|GetIsIdle)
        (Sprite|SetFlipbook (Variables|Default|GetSprite) (Variables|Animations|GetIdle))
        (goto _label)
        (else
          (|Movement))))))